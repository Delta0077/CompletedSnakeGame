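; Game mode for a snake game that spawns food and handles game over.
; On begin play, SpawnFood places a BP_Food at a fixed height and random XY, using 80% of the "Floor"-tagged mesh's extents around world origin.
; Both axes take their minimum from the X extent and maximum from Y.
; GameOver shows WBP_GameOver, pauses the game and switches to UI-only input with a visible cursor.
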(event `SpawnFood`
  ;[1 1 1] SPAWN FOOD FUNCTION
  (bind _outactors (`GameplayStatics.GetAllActorsOfClassWithTag` "/Script/Engine.StaticMeshActor" "Floor"))
  (bind (_origin _boxextent) (`self.GetActorBounds` (`|GetArrayItem` _outactors) false false))
  (`|SpawnActorFromClass` "/Game/Blueprints/BP_Food.BP_Food_C" (`KismetMathLibrary.MakeTransform` (`KismetMathLibrary.MakeVector` (`KismetMathLibrary.RandomFloatInRange` (* (.x _boxextent) -0.8) (* (.y _boxextent) 0.8)) (`KismetMathLibrary.RandomFloatInRange` (* (.x _boxextent) -0.8) (* (.y _boxextent) 0.8)) 120.0)) "Undefined" "OverrideRootScale" null null))

(event `self.ReceiveBeginPlay`
  (`self.SpawnFood`))

(event `GameOver`
  (bind _returnvalue (`|CreateWidget` "/Game/Blueprints/WBP_GameOver.WBP_GameOver_C" (`GameplayStatics.GetPlayerController` 0)))
  (`UserWidget.AddToViewport` _returnvalue 0)
  (`GameplayStatics.SetGamePaused` true)
  (`WidgetBlueprintLibrary.SetInputMode_UIOnlyEx` (`GameplayStatics.GetPlayerController` 0) _returnvalue)
  (set `PlayerController.bShowMouseCursor` true (`GameplayStatics.GetPlayerController` 0)))

(fn `UserConstructionScript`)