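; Player-controlled snake actor for a Snake game that grows a tail and raises the score when EatFood is called.
; Directional inputs turn it only perpendicular to its last actual move, preventing reversals.
; Each Tick moves it one head-mesh width, passing each previous position down the Tails array so segments follow.
; BeginPlay creates the WBP_Main score UI, and new BP_SnakeTail segments spawn behind the head using its mesh.
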(event `InputAction|Up`
  (params (Key :type "Key Structure"))
  (bind _currentmovedir_x (`KismetMathLibrary.BreakVector` (`self.CurrentMoveDir`)))
  ;[1 1 1] INPUT ACTION BINDING With Oneway movement logic
  (:`Pressed`
    (if (== _currentmovedir_x 0.0)
      (set `self.MoveDirection` (1.0 0.0 0.0)))))

(event `self.ReceiveBeginPlay`
  (bind _returnvalue (`StaticMesh.GetBoundingBox` (`StaticMeshComponent.StaticMesh` (`self.Head`))))
  ;[1 1 1] STEP SIZE CALCULATION
  (set `self.StepSize` (- (.x (`.Max` (break `Box` _returnvalue))) (.x (break `Box` _returnvalue))))
  (bind _returnvalue_2 (`|CreateWidget` "/Game/Blueprints/WBP_Main.WBP_Main_C" (`GameplayStatics.GetPlayerController` 0)))
  (bind _output_get (set `self.MainUI` _returnvalue_2))
  (`UserWidget.AddToViewport` _output_get 0))

(event `InputAction|Down`
  (params (Key :type "Key Structure"))
  (bind _currentmovedir_x (`KismetMathLibrary.BreakVector` (`self.CurrentMoveDir`)))
  ;[1 1 1] INPUT ACTION BINDING With Oneway movement logic
  (:`Pressed`
    (if (== _currentmovedir_x 0.0)
      (set `self.MoveDirection` (-1.0 0.0 0.0)))))

(event `self.ReceiveTick`
  (params (DeltaSeconds :type "Float (single-precision)"))
  ;[1 1 1] MOVING FUNCTION
  (set `self.PreviousItemLocation` (`self.K2_GetActorLocation`))
  (`self.K2_AddActorWorldOffset` (* (`self.MoveDirection`) (`self.StepSize`)))
  (set `self.CurrentMoveDir` (- (`self.K2_GetActorLocation`) (`self.PreviousItemLocation`)))
  (for _array_element (`self.Tails`)
    (bind _output_get (set `self.TailCurrentLocation` (`self.K2_GetActorLocation` _array_element)))
    (`self.K2_SetActorLocation` _array_element (`self.PreviousItemLocation`) false false)
    (set `self.PreviousItemLocation` _output_get)))

(event `InputAction|Right`
  (params (Key :type "Key Structure"))
  (bind (_currentmovedir_x _currentmovedir_y) (`KismetMathLibrary.BreakVector` (`self.CurrentMoveDir`)))
  ;[1 1 1] INPUT ACTION BINDING With Oneway movement logic
  (:`Pressed`
    (if (== _currentmovedir_y 0.0)
      (set `self.MoveDirection` (0.0 1.0 0.0)))))

(event `InputAction|Left`
  (params (Key :type "Key Structure"))
  (bind (_currentmovedir_x _currentmovedir_y) (`KismetMathLibrary.BreakVector` (`self.CurrentMoveDir`)))
  ;[1 1 1] INPUT ACTION BINDING With Oneway movement logic
  (:`Pressed`
    (if (== _currentmovedir_y 0.0)
      (set `self.MoveDirection` (0.0 -1.0 0.0)))))

(event `AddScore`
  (bind _result (`/Engine/EditorBlueprintResources/StandardMacros.IncrementInt` (`self.Score`))
    (:`  `
      (bind _aswbp_main (cast `/Game/Blueprints/WBP_Main` (`self.MainUI`)))
      (`/Game/Blueprints/WBP_Main.SetScore` _aswbp_main _result))))

(event `AddTail`
  (bind _returnvalue (`|SpawnActorFromClass` "/Game/Blueprints/BP_SnakeTail.BP_SnakeTail_C" (`KismetMathLibrary.MakeTransform` (- (`self.K2_GetActorLocation`) (* (`self.MoveDirection`) (`self.StepSize`))) (struct) (0.6 0.6 0.6)) "AlwaysSpawn" "OverrideRootScale" null null))
  (`StaticMeshComponent.SetStaticMesh` (`/Game/Blueprints/BP_Trigger.Cube` _returnvalue) (`StaticMeshComponent.StaticMesh` (`self.Head`)))
  (`KismetArrayLibrary.Array_Add` (`self.Tails`) _returnvalue))

(event `EatFood`
  (`self.AddScore`)
  (`self.AddTail`))

(fn `UserConstructionScript`)