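; BP_Food is the food pickup for a snake game.
; When its PlayerOverlapped event fires, it calls EatFood on the player, asks the BP_SnakeGameModeBase game mode to spawn new food, then destroys itself.
; The respawn and destruction run only if the game mode cast succeeds.
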(event `self.PlayerOverlapped`
  (params (Player :type "/Game/Blueprints/BP_Snake Object Reference"))
  (`/Game/Blueprints/BP_Snake.EatFood` Player)
  (bind _asbp_snake_game_mode_base (cast `/Game/Blueprints/BP_SnakeGameModeBase` (`GameplayStatics.GetGameMode`)))
  (`/Game/Blueprints/BP_SnakeGameModeBase.SpawnFood` _asbp_snake_game_mode_base)
  (`self.K2_DestroyActor`))

(fn `UserConstructionScript`
  (`parent.UserConstructionScript`))